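; BP_GameState holds the current match state and runs the countdown timer for the Tumbleweed game.
; ChangeState stores the new state and refills TimeLeft from MaxTimeLeft when entering the first enum state.
; While in that state, Tick decrements TimeLeft and calls EndGame on BP_TumbleweedGameMode whenever it is at or below zero.
; CheckState returns the current state.
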(event `self.ReceiveTick`
  (params (DeltaSeconds :type "Float (single-precision)"))
  (if (`|EnumEquality` (`self.State`) "NewEnumerator0")
    (bind _output_get (set `self.TimeLeft` (- (`self.TimeLeft`) DeltaSeconds)))
    (if (<= _output_get 0.0)
      (bind _asbp_tumbleweed_game_mode (cast `/Game/GameModes/BP_TumbleweedGameMode` (`GameplayStatics.GetGameMode`)))
      (`/Game/GameModes/BP_TumbleweedGameMode.EndGame` _asbp_tumbleweed_game_mode))))

(fn `ChangeState`
  (params (State :type "/Game/Assets/A_GameStates Enum" :default "NewEnumerator0"))
  (bind _output_get (set `self.State` State))
  (if (`|EnumEquality` _output_get "NewEnumerator0")
    (set `self.TimeLeft` (`self.MaxTimeLeft`))))

(fn `CheckState`
  (returns (State :type "/Game/Assets/A_GameStates Enum"))
  (return (`self.State`)))

(fn `UserConstructionScript`)