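; Game mode for the tumbleweed game that runs the flow between main menu, play, game over and restart.
; Each transition changes the BP_GameState state; menu and game over widgets are created here.
; Restart clears widgets, respawns the player pawn and fades out the beach and ghost music.
; StoreAbilities copies the pawn's learned abilities and starting jump and glide values into the game mode at begin play and before each respawn.
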(event `self.ReceiveBeginPlay`
  (`self.StoreAbilities`)
  (bind _asbp_game_state (cast `/Game/Blueprints/BP_GameState` (`GameplayStatics.GetGameState`)))
  (`/Game/Blueprints/BP_GameState.ChangeState` _asbp_game_state "NewEnumerator1")
  (bind _returnvalue (`|CreateWidget` "/Game/HUDs/MainMenu.MainMenu_C"))
  (set `self.Main Menu` _returnvalue)
  (`UserWidget.AddToViewport` _returnvalue 0)
  (`AudioComponent.Stop` (`self.Ghost_BGM`))
  (`AudioComponent.Stop` (`self.Beach_BGM`)))

(event `self.ReceiveTick`
  (params (DeltaSeconds :type "Float (single-precision)")))

(fn `EndGame`
  (bind _asbp_game_state (cast `/Game/Blueprints/BP_GameState` (`GameplayStatics.GetGameState`)))
  (`/Game/Blueprints/BP_GameState.ChangeState` _asbp_game_state "NewEnumerator2")
  (bind _returnvalue (`|CreateWidget` "/Game/HUDs/GameOver.GameOver_C"))
  (set `self.Game Over` _returnvalue)
  (`UserWidget.AddToViewport` _returnvalue 0))

(fn `RestartGame`
  (bind _returnvalue (`GameplayStatics.GetPlayerController` 0))
  (`self.StoreAbilities`)
  (`WidgetLayoutLibrary.RemoveAllWidgets`)
  (bind _asbp_game_state (cast `/Game/Blueprints/BP_GameState` (`GameplayStatics.GetGameState`)))
  (`/Game/Blueprints/BP_GameState.ChangeState` _asbp_game_state "NewEnumerator0")
  (`self.K2_DestroyActor` (`GameplayStatics.GetPlayerPawn` 0))
  (`self.RestartPlayer` _returnvalue)
  (`AudioParameterControllerInterface.SetTriggerParameter` (`self.Beach_BGM`) "FadeOut")
  (`AudioParameterControllerInterface.SetTriggerParameter` (`self.Ghost_BGM`) "FadeOut")
  (`KismetSystemLibrary.PrintText` (`KismetTextLibrary.Conv_VectorToText` (`self.K2_GetActorLocation` (`self.K2_FindPlayerStart` _returnvalue)))))

(fn `StartGame`
  (`Widget.RemoveFromParent` (`self.Main Menu`))
  (bind _asbp_game_state (cast `/Game/Blueprints/BP_GameState` (`GameplayStatics.GetGameState`)))
  (`/Game/Blueprints/BP_GameState.ChangeState` _asbp_game_state "NewEnumerator0"))

(fn `StoreAbilities`
  (bind _asbp_tumbleweed_pawn (cast `/Game/Actors/BP_TumbleweedPawn` (`GameplayStatics.GetPlayerPawn` 0)))
  (set `self.LearnedToJump_GM` (`/Game/Actors/BP_TumbleweedPawn.LearnedToJump` _asbp_tumbleweed_pawn))
  (set `self.LearnedToGlide_GM` (`/Game/Actors/BP_TumbleweedPawn.LearnedToGlide` _asbp_tumbleweed_pawn))
  (set `self.LearnedToWallClimb_GM` (`/Game/Actors/BP_TumbleweedPawn.LearnedToWallClimb` _asbp_tumbleweed_pawn))
  (set `self.StartingJumps_GM` (`/Game/Actors/BP_TumbleweedPawn.Starting Jumps` _asbp_tumbleweed_pawn))
  (set `self.StartingGlide_GM` (`/Game/Actors/BP_TumbleweedPawn.GlideStart` _asbp_tumbleweed_pawn)))

(fn `UserConstructionScript`)