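; A backup tumbleweed player pawn that moves by rotating its physics-driven PlayerSprite.
; The Enhanced Input action IA_MoveByRotate scales its value by RotationalSpeed and applies it as X-axis torque in acceleration-change mode, printing the vector for debugging.
; A jump impulse on the sprite using JumpImpulse is present but never runs, and BeginPlay, overlap and Tick are unused.
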(event `EnhancedInput|/Game/Input/Actions/IA_MoveByRotate`
  (params (ActionValue :type "Float (double-precision)") (ElapsedSeconds :type "Float (double-precision)") (TriggeredSeconds :type "Float (double-precision)") (InputAction :type "InputAction Object Reference" :default "/Game/Input/Actions/IA_MoveByRotate.IA_MoveByRotate"))
  (:`Triggered`
    (bind _result (`/Engine/EditorBlueprintResources/StandardMacros.NegateFloat` (* ActionValue (`self.RotationalSpeed`)))
      (:`  `
        (bind _returnvalue (`KismetMathLibrary.MakeVector` _result))
        (`PrimitiveComponent.AddTorqueInRadians` (`self.PlayerSprite`) _returnvalue "None" true)
        (`KismetSystemLibrary.PrintText` (`KismetTextLibrary.Conv_VectorToText` _returnvalue))))))

(fn `UserConstructionScript`)