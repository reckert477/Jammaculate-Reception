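; Player pawn for a rolling tumbleweed that moves by physics torque and impulses on its sprite, with unlockable jump, glide and wall-climb abilities.
; On BeginPlay it copies abilities and limits from BP_TumbleweedGameMode.
; Holding jump with no jumps left spends glide charges on scaled impulses.
; Overlapping BP_Ground refills jumps and glide (sticky surfaces require wall climb), and leaving it calls the game mode's StoreAbilities.
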(event `self.ReceiveBeginPlay`
  ;[1 1 1] Setup
  (bind _asbp_tumbleweed_game_mode (cast `/Game/GameModes/BP_TumbleweedGameMode` (`GameplayStatics.GetGameMode`)))
  (bind _output_get (set `self.Starting Jumps` (`/Game/GameModes/BP_TumbleweedGameMode.StartingJumps_GM` _asbp_tumbleweed_game_mode)))
  (set `self.RemainingJumps` _output_get)
  (set `self.LearnedToGlide` (`/Game/GameModes/BP_TumbleweedGameMode.LearnedToGlide_GM` _asbp_tumbleweed_game_mode))
  (set `self.LearnedToJump` (`/Game/GameModes/BP_TumbleweedGameMode.LearnedToJump_GM` _asbp_tumbleweed_game_mode))
  (set `self.LearnedToWallClimb` (`/Game/GameModes/BP_TumbleweedGameMode.LearnedToWallClimb_GM` _asbp_tumbleweed_game_mode))
  (bind _startingglide_gm (`/Game/GameModes/BP_TumbleweedGameMode.StartingGlide_GM` _asbp_tumbleweed_game_mode))
  (set `self.GlideStart` _startingglide_gm)
  (set `self.GlideRemaining` _startingglide_gm))

(event `EnhancedInput|/Game/Input/Actions/IA_MoveByRotate`
  (params (ActionValue :type "Float (double-precision)") (ElapsedSeconds :type "Float (double-precision)") (TriggeredSeconds :type "Float (double-precision)") (InputAction :type "InputAction Object Reference" :default "/Game/Input/Actions/IA_MoveByRotate.IA_MoveByRotate"))
  ;[1 1 1] Rolling Horizontally
  (:`Triggered`
    (bind _result (`/Engine/EditorBlueprintResources/StandardMacros.NegateFloat` (* ActionValue (`self.RotationalSpeed`)))
      (:`  `
        (`PrimitiveComponent.AddTorqueInRadians` (`self.PlayerSprite`) (`KismetMathLibrary.MakeVector` _result) "None" true)))))

(event `EnhancedInput|/Game/Input/IA_Jump`
  (params (ActionValue :type Boolean) (ElapsedSeconds :type "Float (double-precision)") (TriggeredSeconds :type "Float (double-precision)") (InputAction :type "InputAction Object Reference" :default "/Game/Input/IA_Jump.IA_Jump"))
  ;[1 1 1] Vertical Movement
  (:`Triggered`
    (if (<= (`self.RemainingJumps`) 0)
      (if (`self.LearnedToGlide`)
        (`self.GlideFunction`))))
  (:`Started`
    (if (`self.LearnedToJump`)
      (if (`self.TouchingGround`)
        (`self.JumpFunction` :!label _label)
        (`KismetSystemLibrary.PrintString` (`KismetStringLibrary.Conv_IntToString` (`self.RemainingJumps`)))
        (elif (> (`self.RemainingJumps`) 0)
          (goto _label))))))

(event `self.Collider.OnComponentBeginOverlap`
  (params (OverlappedComponent :type "PrimitiveComponent Object Reference") (OtherActor :type "Actor Object Reference") (OtherComp :type "PrimitiveComponent Object Reference") (OtherBodyIndex :type Integer) (bFromSweep :type Boolean) (SweepResult :type "HitResult Structure (by ref)"))
  ;[1 1 1] Overlap Detection
  (bind _asbp_ground (cast `/Game/Actors/BP_Ground` OtherActor))
  (if (`self.LearnedToWallClimb`)
    (if (`/Game/Actors/BP_Ground.IsSticky` _asbp_ground)
      (set `self.TouchingGround` true :!label _label_2)
      (set `self.RemainingJumps` (`self.Starting Jumps`))
      (set `self.GlideRemaining` (`self.GlideStart`))
      (else
        (if (`/Game/Actors/BP_Ground.IsGround` _asbp_ground) :!label _label_3
          (goto _label_2))))
    (else
      (goto _label_3))))

(event `self.Collider.OnComponentEndOverlap`
  (params (OverlappedComponent :type "PrimitiveComponent Object Reference") (OtherActor :type "Actor Object Reference") (OtherComp :type "PrimitiveComponent Object Reference") (OtherBodyIndex :type Integer))
  ;[1 1 1] Overlap Detection
  (cast `/Game/Actors/BP_Ground` OtherActor)
  (set `self.TouchingGround` false)
  (bind _asbp_tumbleweed_game_mode (cast `/Game/GameModes/BP_TumbleweedGameMode` (`GameplayStatics.GetGameMode`)))
  (`/Game/GameModes/BP_TumbleweedGameMode.StoreAbilities` _asbp_tumbleweed_game_mode))

(fn `GetBackground`
  (returns (Background :type "Actor Object Reference"))
  (return (`self.CurrentBG`)))

(fn `GlideFunction`
  (if (> (`self.GlideRemaining`) 0)
    (`PrimitiveComponent.AddImpulse` (`self.PlayerSprite`) (`KismetMathLibrary.MakeVector` 0.0 0.0 (* (`self.Jump Impulse`) (`self.HoverVariable`))) "None" false)
    (bind _result (`/Engine/EditorBlueprintResources/StandardMacros.DecrementInt` (`self.GlideRemaining`))
      (:`  `
        (bind _output_get (set `self.GlideRemaining` _result))
        (`KismetSystemLibrary.PrintString` (`KismetStringLibrary.Conv_IntToString` _output_get))))))

(fn `JumpFunction`
  (`PrimitiveComponent.AddImpulse` (`self.PlayerSprite`) (`KismetMathLibrary.MakeVector` 0.0 0.0 (`self.Jump Impulse`)) "None" false)
  (set `self.RemainingJumps` (- (`self.RemainingJumps`) 1)))

(fn `RemoveBackground`
  (set `self.CurrentBG` null))

(fn `SetBackground`
  (params (Background :type "Actor Object Reference"))
  (set `self.CurrentBG` Background))

(fn `UserConstructionScript`)